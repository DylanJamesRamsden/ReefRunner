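; BP_Shark is the shark actor in ReefRunner, adding cosmetic banking to its static mesh as it moves sideways.
; Horizontal movement events set a target roll from the direction, or flag levelling back to zero when movement completes.
; Each Tick interpolates the mesh's world roll at constant speed, keeping pitch and yaw, and clears the active flag on arrival.
; Levelling takes priority over banking until the roll returns to zero.
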(event `self.ReceiveTick`
  (params (DeltaSeconds :type "Float (single-precision)"))
  (`self.CosmeticRotationsTick` DeltaSeconds))

(event `self.OnMovingHorizontally`
  (params (Direction :type "Float (single-precision)"))
  (set `self.HorizontalTargetRoll` (* Direction 15.0))
  (set `self.bRotateHorizontally` true))

(event `self.OnMovingHorizontallyComplete`
  (set `self.bIsLevellingHorizontalRotation` true)
  (set `self.bRotateHorizontally` false))

(event `CosmeticRotationsTick`
  (params (DeltaSeconds :type "Float (single-precision)"))
  (bind _staticmeshcomp (`self.StaticMeshComp`))
  (bind _staticmeshcomp_2 (`self.StaticMeshComp`))
  (bind (_returnvalue_roll _returnvalue_pitch _returnvalue_yaw) (`KismetMathLibrary.BreakRotator` (`SceneComponent.K2_GetComponentRotation` _staticmeshcomp)))
  (bind (_returnvalue_roll_2 _returnvalue_pitch_2 _returnvalue_yaw_2) (`KismetMathLibrary.BreakRotator` (`SceneComponent.K2_GetComponentRotation` _staticmeshcomp_2)))
  (bind _returnvalue (`KismetMathLibrary.RInterpTo_Constant` (`SceneComponent.K2_GetComponentRotation` _staticmeshcomp) (`KismetMathLibrary.MakeRotator` 0.0 _returnvalue_pitch _returnvalue_yaw) DeltaSeconds 50.0))
  (bind _returnvalue_2 (`KismetMathLibrary.RInterpTo_Constant` (`SceneComponent.K2_GetComponentRotation` _staticmeshcomp_2) (`KismetMathLibrary.MakeRotator` (`self.HorizontalTargetRoll`) _returnvalue_pitch_2 _returnvalue_yaw_2) DeltaSeconds 50.0))
  (if (`self.bIsLevellingHorizontalRotation`)
    (`SceneComponent.K2_SetWorldRotation` (`self.StaticMeshComp`) _returnvalue false false)
    (if (`KismetMathLibrary.NearlyEqual_FloatFloat` (.roll _returnvalue))
      (set `self.bIsLevellingHorizontalRotation` false))
    (elif (`self.bRotateHorizontally`)
      (`SceneComponent.K2_SetWorldRotation` (`self.StaticMeshComp`) _returnvalue_2 false false)
      (if (`KismetMathLibrary.NearlyEqual_FloatFloat` (.roll _returnvalue_2) (`self.HorizontalTargetRoll`))
        (set `self.bRotateHorizontally` false)))))

(fn `UserConstructionScript`)