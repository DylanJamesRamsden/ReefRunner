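; Reef Runner character Blueprint that animates the submarine's tilt during horizontal movement.
; Movement events set a target rotation from the horizontal direction, or flag levelling on arrival.
; Tick rotates the Cylinder component toward that target with constant-speed interpolation, clearing each flag once reached.
; Levelling back to zero is slower and takes priority over tilting until it finishes.
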(event `self.ReceiveTick`
  (params (DeltaSeconds :type "Float (single-precision)"))
  (bind _targetrotaion (`self.TargetRotaion`))
  (bind _returnvalue (`KismetMathLibrary.RInterpTo_Constant` (`SceneComponent.K2_GetComponentRotation` (`self.Cylinder`)) (struct) DeltaSeconds 50.0))
  (bind _returnvalue_2 (`KismetMathLibrary.RInterpTo_Constant` (`SceneComponent.K2_GetComponentRotation` (`self.Cylinder`)) _targetrotaion DeltaSeconds 150.0))
  ;[1 1 1] Submarine rotation
  (if (`self.bIsLevellingRotation`)
    ;;[1 1 1] Levels the rotation of the submarine
    (`SceneComponent.K2_SetWorldRotation` (`self.Cylinder`) _returnvalue false false)
    (if (== _returnvalue (struct) :`ErrorTolerance` 0.1)
      (set `self.bIsLevellingRotation` false))
    (else
      ;;[1 1 1] Rotates the submarine in the direction of it's horizontal movement
      (if (`self.bRotateCharacterHorizontally`)
        (`SceneComponent.K2_SetWorldRotation` (`self.Cylinder`) _returnvalue_2 false false)
        (if (== _returnvalue_2 _targetrotaion)
          (set `self.bRotateCharacterHorizontally` false))))))

(event `self.OnMovingHorizontally`
  (params (Direction :type "Vector Structure"))
  (set `self.TargetRotaion` (`KismetMathLibrary.MakeRotator` (* Direction_X 10.0)))
  (set `self.bRotateCharacterHorizontally` true))

(event `self.OnArrivedHorizontally`
  (set `self.TargetRotaion` (struct))
  (set `self.bIsLevellingRotation` true))

(fn `UserConstructionScript`)